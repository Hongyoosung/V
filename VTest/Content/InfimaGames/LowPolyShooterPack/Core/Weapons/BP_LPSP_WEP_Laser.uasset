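; BP_LPSP_WEP_Laser is a weapon laser in the Low Poly Shooter Pack that can be switched on and off.
; Enable and disable events set the Visible flag only when it changes, and its OnRep function calls UpdateVisible, as does BeginPlay.
; UpdateVisible is empty here, so this Blueprint holds the visibility state without applying any visual change itself.
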(event Custom|Event%20Update%20Visible
  ;[0.8831 1 0 1 12] Update Visible
)

(event EventBeginPlay
  ;[1 0.301 0 1 12] Begin Play
  (|CallParentFunction)
  (CallFunction|EventUpdateVisible))

(event EventLPSP-EnableLaser
  ;[0.5348 1 0.009923 1 12] Enable Laser
  (if (not (Variables|Data|GetVisible))
    (Variables|Data|SetVisible true)))

(event EventLPSP-DisableLaser
  ;[0.069 1 0.3722 1 12] Disable Laser
  (if (Variables|Data|GetVisible)
    (Variables|Data|SetVisible false)))

(fn ConstructionScript
  (|CallParentFunction))

(fn OnRepVisible
  (CallFunction|EventUpdateVisible))