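; Weapon laser sight attachment that manages two parts, a dot and a beam.
; Property updates are stored and passed to both parts.
; Visibility changes spawn the dot through a server event if it is missing and should be visible, then apply visibility to both parts.
; Unequipping the parent destroys the dot through a server event, while the beam's visibility event has no server prefix.
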(event EventLPSP-PieceParentEquipped)

(event EventLPSP-PieceParentUnequipped
  (Default|EventServerDestroy (Variables|Default|GetDot)))

(event EventEventUpdateVisible
  (|CallParentFunction)
  (Utilities|FlowControl|Sequence
    (:then_0
      (if (not (Default|Exists (Variables|Default|GetDot)))
        (if (Variables|Default|GetVisible)
          (Default|EventServerSpawn (Variables|Default|GetDot)))))
    (:then_1
      (Default|EventServerSetVisibility (Variables|Default|GetDot) (Variables|Default|GetVisible))
      (Default|EventSetVisibility (Variables|Default|GetBeam) (Variables|Default|GetVisible)))))

(event EventUpdateLasersightProperties
  (params (Properties :type S%20Lasersight%20Structure))
  (Variables|Default|SetProperties Properties)
  (Default|EventUpdateProperties (Variables|Default|GetDot) (Variables|Default|GetProperties))
  (Default|EventUpdateProperties (Variables|Default|GetBeam) (Variables|Default|GetProperties)))

(fn ConstructionScript
  (|CallParentFunction))