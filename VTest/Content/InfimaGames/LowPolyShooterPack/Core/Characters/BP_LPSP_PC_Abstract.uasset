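; Abstract player controller for the Low Poly Shooter Pack that starts the player spawn flow.
; On BeginPlay, it either creates the spawn menu widget for the local controller when SpawnLoadoutMenu is enabled, or requests a spawn immediately without attachment overrides.
; The SpawnPlayer server event forwards loadout, attachment override and inventory data to the game mode through a message call, leaving the actual spawning there.
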(event Custom|Event%20Show%20Spawn%20Menu
  ;[1 0.07939 0 1 12] Show Spawn Menu
  (bind _returnvalue (UserInterface|CreateWidget (Variables|Config|GetSpawn%20Menu%20Class) self))
  (UserInterface|Viewport|AddtoViewport _returnvalue 0))

(event Custom|Event%20%28Server%29%20Spawn%20Player
  (params (Override%20Attachments :type Boolean) (Loadout :type S%20LPSP%20Loadout%20Structure) (Inventory%20Data :type Data%20Table%20Object%20Reference))
  ;[1 0.9481 0 1 12] Spawn Player
  (Class|BPILPSPGM|LPSP-SpawnPlayer(Message) (Game|GetGameMode) self Inventory%20Data Override%20Attachments Loadout))

(event EventBeginPlay
  ;[0.9123 1 0 1 12] Begin Play
  (CallFunction|TryShowSpawnMenu))

(fn ConstructionScript)

(fn TryShowSpawnMenu
  (Utilities|FlowControl|Sequence
    (:then_0
      (if (Variables|Config|GetSpawn%20Loadout%20Menu)
        (if (Pawn|IsLocalPlayerController)
          (CallFunction|EventShowSpawnMenu))
        (else
          (CallFunction|Event(Server)SpawnPlayer false))))
    (:then_1
      (return))))