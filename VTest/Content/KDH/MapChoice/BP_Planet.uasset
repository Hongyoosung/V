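; BP_Planet is a clickable planet actor in MapChoice that the mouse spins.
; While the left button is held, MouseX and MouseY input apply inverted yaw and pitch to the Planet component's relative rotation.
; Clicking the Company1 component streams in TestLevel.
; An inertial spin built from HandleDrag and HandleRotation, with damped velocity, remains in the graph but is never driven, as Tick is empty.
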(event OnClicked(company1)
  (params (TouchedComponent :type Primitive%20Component%20Object%20Reference) (ButtonPressed :type Key%20Structure :default "None"))
  (Game|LoadStreamLevel(byName) "TestLevel" true))

(event Custom|HandleRotation
  (params (Delta%20Time :type Float%20%28double-precision%29))
  (Class|Actor|AddActorWorldRotation (Math|Rotator|MakeRotator 0.0 0.0 (* Delta%20Time (Variables|Default|GetRotateVelocity))))
  (if (or (< (Variables|Default|GetRotateVelocity) -0.1) (> (Variables|Default|GetRotateVelocity) 0.1))
    (Variables|Default|SetRotateVelocity (* (Variables|Default|GetRotateVelocity) 0.9))
    (Variables|Default|SetdragSumX (* (Variables|Default|GetdragSumX) 0.9))))

(event Custom|HandleDrag
  (params (Delta%20Time :type Float%20%28double-precision%29))
  (if (Variables|Default|GetisDrag)
    (bind _output_get (Variables|Default|SetdragSumX (- (Variables|Default|GetdragSumX) (Class|Actor|GetInputAxisKeyValue))))
    (Variables|Default|SetRotateVelocity (+ (Variables|Default|GetRotateVelocity) (* (* _output_get Delta%20Time) 9e+01)))
    (else
      (Variables|Default|SetdragSumX 0.0))))

(event EventBeginPlay)

(event Collision|EventActorBeginOverlap
  (params (OtherActor :type Actor%20Object%20Reference)))

(event EventTick
  (params (DeltaSeconds :type Float%20%28single-precision%29)))

(event Input|MouseEvents|MouseY
  (params (AxisValue :type Float%20%28single-precision%29))
  ;[1 1 1] Y-AXIS ROTATE
  (if (Game|Player|IsInputKeyDown (Game|GetPlayerController 0) "LeftMouseButton")
    (Transformation|SetRelativeRotation (Variables|Actor|GetPlanet) (Math|Rotator|CombineRotators (Variables|/Script/Engine.SceneComponent|GetRelativeRotation (Variables|Actor|GetPlanet)) (Math|Rotator|MakeRotator 0.0 (* AxisValue -1.0) 0.0)) false false)))

(event Input|MouseEvents|MouseX
  (params (AxisValue :type Float%20%28single-precision%29))
  ;[1 1 1] X-AXIS ROTATE
  (if (Game|Player|IsInputKeyDown (Game|GetPlayerController 0) "LeftMouseButton")
    (Transformation|SetRelativeRotation (Variables|Actor|GetPlanet) (Math|Rotator|CombineRotators (Variables|/Script/Engine.SceneComponent|GetRelativeRotation (Variables|Actor|GetPlanet)) (Math|Rotator|MakeRotator 0.0 0.0 (* AxisValue -1.0))) false false)))

(fn ConstructionScript)